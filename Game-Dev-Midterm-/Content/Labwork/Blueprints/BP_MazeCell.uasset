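; BP_MazeCell is a maze building block whose construction script builds a scaled floor, optional walls and ceiling from grid size and wall height.
; A ceiling with positive intensity also gets a colored point light.
; At BeginPlay it binds to the player character's maze gate event; leaving recolors a valid PointLight to the character's color, disables input and quits after a delay.
; The death-screen widget logic is unconnected.
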(event `self.ReceiveBeginPlay`
  (bind _asbp_third_person_character (cast `/Game/Labwork/Blueprints/BP_ThirdPersonCharacter` (`GameplayStatics.GetPlayerPawn` 0)))
  (set `self.As BP Third Person Character` _asbp_third_person_character)
  (add `/Game/Labwork/Blueprints/BP_ThirdPersonCharacter.Maze_Gate` _asbp_third_person_character (delegate `MazeGate_Event`)))

(event `MazeGate_Event`
  (params (`Isinside?` :type Boolean))
  (bind _pointlight (`self.PointLight`))
  (if (not `Isinside?`)
    (`/Engine/EditorBlueprintResources/StandardMacros.IsValid` _pointlight
      (:`Is Valid`
        (`LightComponent.SetLightColor` _pointlight (`/Game/Labwork/Blueprints/BP_ThirdPersonCharacter.LightColor` (`self.As BP Third Person Character`)) true)
        (`self.DisableInput` (`GameplayStatics.GetPlayerCharacter` 0) (`GameplayStatics.GetPlayerController` 0))
        (`KismetSystemLibrary.Delay` 2.0)
        (`KismetSystemLibrary.QuitGame` null "Quit")))))

(fn `UserConstructionScript`
  (locals (WallLength :type "Float (double-precision)") (WallThickness :type "Float (double-precision)"))
  (bind _gridsize (`self.GridSize`))
  (bind _walllength (`local.WallLength`))
  (bind _walllength_2 (`local.WallLength`))
  (bind _returnvalue (* (`local.WallLength`) 0.5))
  (set `local.WallLength` _gridsize)
  (set `local.WallThickness` (* _gridsize 0.1))
  (`SceneComponent.SetRelativeScale3D` (`self.Floor`) (`self.SizeToCubeScale` (`KismetMathLibrary.MakeVector` _walllength_2 _walllength_2 (`local.WallThickness`))))
  (if (`self.WestWall`)
    (`AddComponent|NODE_AddStaticMeshComponent-1` :`RelativeTransform` (`KismetMathLibrary.MakeTransform` (0.0 0.0 0.0) (struct) (`self.SizeToCubeScale` (`KismetMathLibrary.MakeVector` (`local.WallLength`) (`local.WallThickness`) (`self.WallHeight`))))))
  (if (`self.SouthWall`)
    (`AddComponent|NODE_AddStaticMeshComponent-2` :`RelativeTransform` (`KismetMathLibrary.MakeTransform` (0.0 0.0 0.0) (struct) (`self.SizeToCubeScale` (`KismetMathLibrary.MakeVector` (`local.WallThickness`) (`local.WallLength`) (`self.WallHeight`))))))
  (if (`self.NorthWall`)
    (`AddComponent|NODE_AddStaticMeshComponent-3` :`RelativeTransform` (`KismetMathLibrary.MakeTransform` (`KismetMathLibrary.MakeVector` (- (`local.WallLength`) (`local.WallThickness`))) (struct) (`self.SizeToCubeScale` (`KismetMathLibrary.MakeVector` (`local.WallThickness`) (`local.WallLength`) (`self.WallHeight`))))))
  (if (`self.EastWall`)
    (`AddComponent|NODE_AddStaticMeshComponent-4` :`RelativeTransform` (`KismetMathLibrary.MakeTransform` (`KismetMathLibrary.MakeVector` 0.0 (- (`local.WallLength`) (`local.WallThickness`))) (struct) (`self.SizeToCubeScale` (`KismetMathLibrary.MakeVector` (`local.WallLength`) (`local.WallThickness`) (`self.WallHeight`))))))
  (if (`self.Ceiling`)
    (`AddComponent|NODE_AddStaticMeshComponent-5` :`RelativeTransform` (`KismetMathLibrary.MakeTransform` (`KismetMathLibrary.MakeVector` 0.0 0.0 (`self.WallHeight`)) (struct) (`self.SizeToCubeScale` (`KismetMathLibrary.MakeVector` _walllength _walllength (`local.WallThickness`)))))
    (if (> (`self.LightIntensity`) 0.0)
      (bind _returnvalue_2 (`AddComponent|NODE_AddPointLightComponent-0` :`RelativeTransform` (`KismetMathLibrary.MakeTransform` (`KismetMathLibrary.MakeVector` _returnvalue _returnvalue (* (`self.WallHeight`) 0.9)))))
      (`LightComponent.SetLightColor` _returnvalue_2 (`self.LightColor`) true)
      (`LightComponent.SetIntensity` _returnvalue_2 (`self.LightIntensity`)))))