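; BP_Door is a locked door for a maze game that slides open when interacted with while the player has the matching key value.
; On BeginPlay it caches GM_Maze, and Interact opens only if that game mode's Keys exactly equals KeyNumber, otherwise printing a message.
; Despite its name, the DoorRotate timeline lerps the door's relative location from StartLocation to FinishLocation.
; The construction script applies a configurable material to the door.
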(event `self.ReceiveBeginPlay`
  (bind _asgm_maze (cast `/Game/Labwork/Blueprints/GM_Maze` (`GameplayStatics.GetGameMode`)))
  (set `self.As GM Maze` _asgm_maze))

(event `/Game/Labwork/Blueprints/BPI_Interactable.Interact`
  (if (== (`/Game/Labwork/Blueprints/GM_Maze.Keys` (`self.As GM Maze`)) (`self.KeyNumber`))
    (bind (_direction _newtrack_0) (`Timeline|Door Rotate`)
      (:`Update`
        (`SceneComponent.K2_SetRelativeLocation` (`self.Door`) (`KismetMathLibrary.VLerp` (`self.StartLocation`) (`self.FinishLocation`) _newtrack_0) false false)))
    (else
      (`KismetSystemLibrary.PrintString` "You don't have the correct Key"))))

(fn `UserConstructionScript`
  (`PrimitiveComponent.SetMaterial` (`self.Door`) 0 (`self.Material`)))