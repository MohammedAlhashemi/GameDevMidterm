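; BP_Key is a key pickup actor for the maze game mode GM_Maze.
; It caches the game mode on BeginPlay and applies a configurable material to its Key component in the construction script.
; On Interact, it sets the game mode's Keys value to its own KeyNumber, overwriting the previous one.
; It then prints an acquired message using the matching entry in Names and destroys itself.
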(event `self.ReceiveBeginPlay`
  (bind _asgm_maze (cast `/Game/Labwork/Blueprints/GM_Maze` (`GameplayStatics.GetGameMode`)))
  (set `self.As GM Maze` _asgm_maze))

(event `/Game/Labwork/Blueprints/BPI_Interactable.Interact`
  (bind _output_get (set `/Game/Labwork/Blueprints/GM_Maze.Keys` (`self.KeyNumber`) (`self.As GM Maze`)))
  (`KismetSystemLibrary.PrintString` (`KismetStringLibrary.Concat_StrStr` (`|GetArrayItem` (`self.Names`) _output_get) " Key" " Acquired"))
  (`self.K2_DestroyActor`))

(fn `UserConstructionScript`
  (`PrimitiveComponent.SetMaterial` (`self.Key`) 0 (`self.Material`)))