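; Pickup-style trap deactivator actor that disables traps of a configured type in the maze game.
; When the third-person character overlaps its box, it passes its TrapTypes value to GM_Maze's CallDestroyTrap, then destroys itself and prints a confirmation message.
; The construction script applies an exposed material to its static mesh.
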(event `self.Box.OnComponentBeginOverlap`
  (params (OverlappedComponent :type "PrimitiveComponent Object Reference") (OtherActor :type "Actor Object Reference") (OtherComp :type "PrimitiveComponent Object Reference") (OtherBodyIndex :type Integer) (bFromSweep :type Boolean) (SweepResult :type "HitResult Structure (by ref)"))
  (cast `/Game/Labwork/Blueprints/BP_ThirdPersonCharacter` OtherActor)
  (bind _asgm_maze (cast `/Game/Labwork/Blueprints/GM_Maze` (`GameplayStatics.GetGameMode`)))
  (`/Game/Labwork/Blueprints/GM_Maze.DestroyTrap` _asgm_maze (`self.TrapTypes`))
  (`self.K2_DestroyActor`)
  (`KismetSystemLibrary.PrintString` "You Deactivated a trap!"))

(fn `UserConstructionScript`
  (`PrimitiveComponent.SetMaterial` (`self.StaticMesh`) 0 (`self.Material`)))