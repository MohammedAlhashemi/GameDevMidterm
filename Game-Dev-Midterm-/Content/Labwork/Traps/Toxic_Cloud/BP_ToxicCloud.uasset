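; Toxic cloud trap actor for the maze game that deals repeated radial damage around its location.
; Tick runs through a half-second Delay, so full, falloff-free damage pulses roughly twice a second within DamageRadius.
; On BeginPlay it binds to the GM_Maze game mode's DestroyTrap event and destroys itself when the broadcast trap type matches its hard-coded enum value.
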(event `self.ReceiveTick`
  (params (DeltaSeconds :type "Float (single-precision)"))
  (`KismetSystemLibrary.Delay` 0.5)
  (`GameplayStatics.ApplyRadialDamage` :`BaseDamage` 30.0 :`Origin` (`self.K2_GetActorLocation`) :`DamageRadius` (`self.Damage Radius`) :`DamageCauser` null :`InstigatedByController` null :`bDoFullDamage` true))

(event `self.ReceiveBeginPlay`
  (bind _asgm_maze (cast `/Game/Labwork/Blueprints/GM_Maze` (`GameplayStatics.GetGameMode`)))
  (add `/Game/Labwork/Blueprints/GM_Maze.DestroyTrap` _asgm_maze (delegate `DestroyTrap`)))

(event `DestroyTrap`
  (params (Traps :type "/Game/Labwork/Traps/E_Traps Enum" :default "NewEnumerator0"))
  (if (`|EnumEquality` Traps "NewEnumerator2")
    (`self.K2_DestroyActor`)))

(fn `UserConstructionScript`)