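; BP_SpinningBlade is a rotating blade trap that damages the player character in the maze.
; Either of two damage boxes applies fixed damage one second after BP_ThirdPersonCharacter begins overlapping it, without rechecking the overlap.
; On BeginPlay it binds to GM_Maze's destroy-trap event, which stops rotation and removes both boxes when the trap type matches.
; The construction script applies the Material variable to the blade mesh.
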(event `self.ReceiveBeginPlay`
  (bind _asgm_maze (cast `/Game/Labwork/Blueprints/GM_Maze` (`GameplayStatics.GetGameMode`)))
  (add `/Game/Labwork/Blueprints/GM_Maze.DestroyTrap` _asgm_maze (delegate `DestroyTrap`)))

(event `DestroyTrap`
  (params (Traps :type "/Game/Labwork/Traps/E_Traps Enum" :default "NewEnumerator0"))
  (if (`|EnumEquality` Traps "NewEnumerator1")
    (`ActorComponent.Deactivate` (`self.RotatingMovement`))
    (`ActorComponent.K2_DestroyComponent` (`self.Damagebox`))
    (`ActorComponent.K2_DestroyComponent` (`self.Damagebox1`))))

(event `self.Damagebox.OnComponentBeginOverlap`
  (params (OverlappedComponent :type "PrimitiveComponent Object Reference") (OtherActor :type "Actor Object Reference") (OtherComp :type "PrimitiveComponent Object Reference") (OtherBodyIndex :type Integer) (bFromSweep :type Boolean) (SweepResult :type "HitResult Structure (by ref)"))
  (bind _asbp_third_person_character (cast `/Game/Labwork/Blueprints/BP_ThirdPersonCharacter` OtherActor))
  (`KismetSystemLibrary.Delay` 1.0)
  (`GameplayStatics.ApplyDamage` _asbp_third_person_character 40.0))

(event `self.Damagebox1.OnComponentBeginOverlap`
  (params (OverlappedComponent :type "PrimitiveComponent Object Reference") (OtherActor :type "Actor Object Reference") (OtherComp :type "PrimitiveComponent Object Reference") (OtherBodyIndex :type Integer) (bFromSweep :type Boolean) (SweepResult :type "HitResult Structure (by ref)"))
  (bind _asbp_third_person_character (cast `/Game/Labwork/Blueprints/BP_ThirdPersonCharacter` OtherActor))
  (`KismetSystemLibrary.Delay` 1.0)
  (`GameplayStatics.ApplyDamage` _asbp_third_person_character 40.0))

(fn `UserConstructionScript`
  (`PrimitiveComponent.SetMaterial` (`self.SpinningBlade`) 0 (`self.Material`)))