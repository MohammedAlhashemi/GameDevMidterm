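; BP_Pendulum is a swinging trap that deals heavy damage to a BP_ThirdPersonCharacter entering its Box.
; A timeline lerps the Scene's relative rotation back and forth, reversing each time it finishes to loop endlessly.
; Every timeline update also binds to GM_Maze's DestroyTrap event, which destroys the actor when the trap enum matches its first entry.
; The construction script applies a configurable material to the Pendulum.
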(event `self.ReceiveBeginPlay`
  (bind (_direction _pendswing) (`Timeline|PendulumSwing` :!label _label)
    (:`Update`
      (`SceneComponent.K2_SetRelativeRotation` (`self.Scene`) (`KismetMathLibrary.RLerp` (struct :`Pitch` -20.0) (struct :`Pitch` 20.0) _pendswing) false false)
      (bind _asgm_maze (cast `/Game/Labwork/Blueprints/GM_Maze` (`GameplayStatics.GetGameMode`)))
      (add `/Game/Labwork/Blueprints/GM_Maze.DestroyTrap` _asgm_maze (delegate `DestroyTrap`)))
    (:`Finished`
      (if (`|EnumEquality` _direction "Forward")
        (goto _label :!via `Reverse`)
        (else
          (goto _label))))))

(event `DestroyTrap`
  (params (Traps :type "/Game/Labwork/Traps/E_Traps Enum" :default "NewEnumerator0"))
  (if (`|EnumEquality` Traps "NewEnumerator0")
    (`self.K2_DestroyActor`)))

(event `self.Box.OnComponentBeginOverlap`
  (params (OverlappedComponent :type "PrimitiveComponent Object Reference") (OtherActor :type "Actor Object Reference") (OtherComp :type "PrimitiveComponent Object Reference") (OtherBodyIndex :type Integer) (bFromSweep :type Boolean) (SweepResult :type "HitResult Structure (by ref)"))
  (bind _asbp_third_person_character (cast `/Game/Labwork/Blueprints/BP_ThirdPersonCharacter` OtherActor))
  (`GameplayStatics.ApplyDamage` _asbp_third_person_character 100.0))

(fn `UserConstructionScript`
  (`PrimitiveComponent.SetMaterial` (`self.Pendulum`) 0 (`self.Material`)))